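; BP_dot is a player character that runs along world X and shifts along Y within a clamped depth band, like a 2.5D side-scroller.
; Axis inputs drive movement, and a sign change against the stored Direccion flips the mesh to face the new way.
; It pushes jump, crouch and movement flags straight into dot_animbp, clearing jump on landing and movement at zero velocity.
; The swimming flag is only reset at BeginPlay.
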(event `self.ReceiveBeginPlay`
  (bind _asdot_animbp (cast `/Game/Assets/dot_animbp` (`SkeletalMeshComponent.GetAnimInstance` (`self.Mesh`))))
  (bind _output_get (set `self.AnimBP` _asdot_animbp))
  (`|ExecutionSequence`
    (:`then_0`
      (set `/Game/Assets/dot_animbp.isJumping` false _output_get))
    (:`then_1`
      (set `/Game/Assets/dot_animbp.isCrouching` false _output_get))
    (:`then_2`
      (set `/Game/Assets/dot_animbp.isMoving` false _output_get))
    (:`then_3`
      (set `/Game/Assets/dot_animbp.isSwimming` false _output_get))
    (:`then_4`
      (set `self.direccion` 1.0))))

(event `InputAction|Crouch`
  (params (Key :type "Key Structure"))
  (bind _animbp (`self.AnimBP`))
  (:`Pressed`
    (set `/Game/Assets/dot_animbp.isCrouching` true _animbp))
  (:`Released`
    (set `/Game/Assets/dot_animbp.isCrouching` false _animbp)))

(event `InputAction|jump`
  (params (Key :type "Key Structure"))
  (:`Pressed`
    (`self.Jump`)
    (set `/Game/Assets/dot_animbp.isJumping` true (`self.AnimBP`))))

(event `self.K2_OnMovementModeChanged`
  (params (PrevMovementMode :type "EMovementMode Enum" :default "MOVE_None") (NewMovementMode :type "EMovementMode Enum" :default "MOVE_None") (PrevCustomMode :type Byte) (NewCustomMode :type Byte))
  (`|ExecutionSequence`
    (:`then_0`
      (if (and (`|EnumEquality` PrevMovementMode "MOVE_Falling") (`|EnumEquality` NewMovementMode "MOVE_Walking"))
        (set `/Game/Assets/dot_animbp.isJumping` false (`self.AnimBP`))))))

(event `InputAxis|Back`
  (params (AxisValue :type "Float (single-precision)"))
  (`self.AddMovementInput` (0.0 10.0 0.0) AxisValue)
  (set `/Game/Assets/dot_animbp.isMoving` true (`self.AnimBP`))
  (`self.K2_SetActorLocation` (`KismetMathLibrary.MakeVector` (.x (`self.K2_GetActorLocation`)) (`KismetMathLibrary.FClamp` (.y (`self.K2_GetActorLocation`)) 80.0 160.0) (.z (`self.K2_GetActorLocation`)))))

(event `InputAxis|Forward`
  (params (AxisValue :type "Float (single-precision)"))
  (bind _animbp (`self.AnimBP`))
  (bind _mesh (`self.Mesh`))
  (bind _velocity (`MovementComponent.Velocity` (`self.CharacterMovement`)))
  (`|ExecutionSequence`
    (:`then_0`
      (`self.AddMovementInput` (10.0 0.0 0.0) AxisValue)
      (set `/Game/Assets/dot_animbp.isMoving` true _animbp))
    (:`then_1`
      (if (== (`KismetMathLibrary.Dot_VectorVector` _velocity _velocity) 0.0)
        (set `/Game/Assets/dot_animbp.isMoving` false _animbp)))
    (:`then_2`
      (if (< (* AxisValue (`self.direccion`)) 0.0)
        (bind _output_get (set `self.direccion` AxisValue))
        (if (> _output_get 0.0)
          (`SceneComponent.K2_SetWorldRotation` _mesh (struct :`Yaw` -90.0) false false)
          (else
            (`SceneComponent.K2_SetWorldRotation` _mesh (struct :`Yaw` 90.0) false false)))))))

(fn `UserConstructionScript`)